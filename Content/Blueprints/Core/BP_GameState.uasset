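; Game state that acts as a relay for scoring, respawning and combat audio in a multiplayer game with blocking.
; Multicast events increment kills and deaths in each player state's scorecard struct, and remove departing clients from PlayerArray.
; Respawn and model-removal requests forward to BP_EGGameplayGM, with respawns also counting a death, while cursor colour changes go to the defender's controller.
; Further multicasts play block, hit and death sounds at locations, adding a 2D cheer on death.
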(event Custom|GS_RemovePlayerModel
  (params (OutPlayer :type BP%20EG%20Player%20Controller%20Object%20Reference))
  (bind _asbp_eggameplay_gm (Utilities|Casting|CastToBP_EGGameplayGM (Game|GetGameMode)))
  (Default|RemovePlayerModel _asbp_eggameplay_gm OutPlayer))

(event Custom|GS_RespawnPlayer
  (params (In%20Player :type BP%20EG%20Player%20Controller%20Object%20Reference))
  ;[1 0.3435 0] Respawn Player Event to call on the Game Mode
  (bind _asbp_eggameplay_gm (Utilities|Casting|CastToBP_EGGameplayGM (Game|GetGameMode))
    (:then
      (Default|RespawnRequest _asbp_eggameplay_gm In%20Player)
      (CallFunction|MulticastIncrementPlayerDeath (Variables|/Script/Engine.Controller|GetPlayerState In%20Player)))
    (:CastFailed
      (Development|PrintString "Respawn Request Cast Failed" true true "(R=0.000000,G=0.660000,B=1.000000,A=1.000000)" 1e+01))))

(event Custom|Multicast_WB
  (params (SoundLocation :type Vector))
  ;[0.4775 0.7954 1] Play Sounds at Location
  (Audio|PlaySoundatLocation "/Game/Blueprints/Sounds/SwordClash/WrongBlock_Cue.WrongBlock_Cue" SoundLocation "0, 0, 0" 1.0 1.0 0.0 0 0 0 0))

(event Custom|Multicast_PB
  (params (SoundLocation :type Vector))
  ;[0.4775 0.7954 1] Play Sounds at Location
  (Audio|PlaySoundatLocation "/Game/Blueprints/Sounds/SwordClash/PerfectBlock_Cue.PerfectBlock_Cue" SoundLocation "0, 0, 0" 1.0 1.0 0.0 0 0 0 0))

(event Custom|Multicast_IB
  (params (SoundLocation :type Vector))
  ;[0.4775 0.7954 1] Play Sounds at Location
  (Audio|PlaySoundatLocation "/Game/Blueprints/Sounds/SwordClash/ImperfectBlock_Cue.ImperfectBlock_Cue" SoundLocation "0, 0, 0" 1.0 1.0 0.0 0 0 0 0))

(event Custom|Multicast_DH
  (params (Location :type Vector))
  ;[0.4775 0.7954 1] Play Sounds at Location
  (Audio|PlaySoundatLocation "/Game/Blueprints/Sounds/DirectHit/DH_Cue.DH_Cue" Location "0, 0, 0" 1.0 1.0 0.0 0 0 0 0))

(event Custom|Server_RemoveClient
  (params (OutgoingController :type BP%20EG%20Player%20Controller%20Object%20Reference))
  (CallFunction|MulticastRemoveClient OutgoingController))

(event Custom|Multicast_Death
  (params (Location :type Vector))
  ;[0.4775 0.7954 1] Play Sounds at Location
  (Audio|PlaySoundatLocation "/Game/Blueprints/Sounds/Death/Death_Cue.Death_Cue" Location "0, 0, 0" 1.0 1.0 0.0 0 0 0 0)
  (Audio|PlaySound2D "/Game/Blueprints/Sounds/Ambient/Cheering_Cue.Cheering_Cue" 1.0 1.0 0.0 0 0))

(event Custom|Multicast_RemoveClient
  (params (OutgoingController :type BP%20EG%20Player%20Controller%20Object%20Reference))
  (bind _returnvalue (Utilities|Array|RemoveItem (Variables|Default|GetPlayerArray) (Variables|/Script/Engine.Controller|GetPlayerState OutgoingController)))
  (if _returnvalue
    (Development|PrintString "Player Removed from the Array" true true "(R=1.000000,G=0.000000,B=0.887047,A=1.000000)")
    (else
      (Development|PrintString "Failed to Remove Player" true true "(R=1.000000,G=0.081652,B=0.000000,A=1.000000)"))))

(event Custom|Multicast_IncrementPlayerDeath
  (params (PlayerState :type Player%20State%20Object%20Reference))
  ;[0 0.5715 1] Increment Scorecard
  (bind _asbp_egplayer_state (Utilities|Casting|CastToBP_EGPlayerState PlayerState))
  (Utilities|Struct|SetmembersinBP_ScorecardInfo (Variables|/Game/Blueprints/Core/PlayerState/BP_EGPlayerState.BP_EGPlayerState_C|GetScoreCardInfo _asbp_egplayer_state) (+ (Utilities|Struct|BreakBP_ScorecardInfo (Variables|/Game/Blueprints/Core/PlayerState/BP_EGPlayerState.BP_EGPlayerState_C|GetScoreCardInfo _asbp_egplayer_state)) 1)))

(event Custom|Server_ChangeDefendingPlayerCursor
  (params (DefendingChar :type BP%20EG%20Base%20Character%20Object%20Reference) (ColourInt :type Integer))
  ;[1 1 1] Change cursor through game state
  (bind _asbp_egplayer_controller (Utilities|Casting|CastToBP_EGPlayerController (Pawn|GetController DefendingChar)))
  (Default|ChangeCursorColour _asbp_egplayer_controller ColourInt))

(event Custom|Multicast_IncrementPlayerKills
  (params (PlayerState :type Player%20State%20Object%20Reference))
  ;[0 0.5715 1] Increment Scorecard
  (bind _asbp_egplayer_state (Utilities|Casting|CastToBP_EGPlayerState PlayerState)
    (:then
      (Utilities|Struct|SetmembersinBP_ScorecardInfo (Variables|/Game/Blueprints/Core/PlayerState/BP_EGPlayerState.BP_EGPlayerState_C|GetScoreCardInfo _asbp_egplayer_state) (+ (Utilities|Struct|BreakBP_ScorecardInfo (Variables|/Game/Blueprints/Core/PlayerState/BP_EGPlayerState.BP_EGPlayerState_C|GetScoreCardInfo _asbp_egplayer_state)) 1)))
    (:CastFailed
      (Development|PrintString "FAILED TO CAST TO EGPLAYERSTATE"))))

(event Custom|Server_IncrementPlayerKills
  (params (PlayerController :type BP%20EG%20Player%20Controller%20Object%20Reference))
  ;[0 0.5715 1] Increment Scorecard
  (CallFunction|MulticastIncrementPlayerKills (Variables|/Script/Engine.Controller|GetPlayerState PlayerController)))

(event EventBeginPlay)

(event EventTick
  (params (DeltaSeconds :type Float%20%28single-precision%29)))

(fn ConstructionScript)
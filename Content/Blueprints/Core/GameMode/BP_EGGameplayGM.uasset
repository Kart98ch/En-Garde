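; BP_EGGameplayGM is the gameplay game mode that manages players joining, respawning and leaving a multiplayer match.
; PostLogin tracks each BP_EGPlayerController, spawns its pawn, sets game-only input and creates its cursor, while logout destroys the pawn and untracks the controller.
; SpawnPlayer, shared with authority-checked respawn requests, replaces any existing pawn with a possessed BP_EGBaseCharacter at a random PlayerStart.
; Tick prints the connected player count as debug output.
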(event Custom|RespawnRequest
  (params (PlayerController :type BP%20EG%20Player%20Controller%20Object%20Reference))
  ;[0.08907 1 0] Respawn Request - Recieves request from player controller to respawn their pawn after death
  (Utilities|IsValid PlayerController
    (:Is%20Valid
      (Networking|SwitchHasAuthority
        (:Authority
          (CallFunction|SpawnPlayer PlayerController))))))

(event Custom|RemovePlayerModel
  (params (OutPlayer :type BP%20EG%20Player%20Controller%20Object%20Reference))
  (bind _returnvalue (Pawn|GetControlledPawn OutPlayer))
  (Utilities|IsValid _returnvalue
    (:Is%20Valid
      (Actor|DestroyActor _returnvalue)
      (Default|LeaveGame OutPlayer))))

(event EventTick
  (params (DeltaSeconds :type Float%20%28single-precision%29))
  (bind _asbp_game_state (Utilities|Casting|CastToBP_GameState (Game|GetGameState)))
  (Development|PrintString (Utilities|String|Append "Players Connected: " (Utilities|String|ToString(Integer) (Utilities|Array|Length (Variables|/Script/Engine.GameStateBase|GetPlayerArray _asbp_game_state)))) true true "(R=0.000000,G=0.660000,B=1.000000,A=1.000000)" 0.0))

(event EventPostLogin
  (params (NewPlayer :type Player%20Controller%20Object%20Reference))
  ;[0 0.4926 1] OnPostLogin - Adds to PlayerController array and spawns joining players
  (bind _asbp_egplayer_controller (Utilities|Casting|CastToBP_EGPlayerController NewPlayer))
  (Utilities|Array|Add (Variables|Default|GetPlayer%20Controllers) _asbp_egplayer_controller)
  (CallFunction|SpawnPlayer NewPlayer)
  (Input|SetInputModeGameOnly NewPlayer false)
  (Default|CreateCursor _asbp_egplayer_controller))

(event EventOnLogout
  (params (ExitingController :type Controller%20Object%20Reference))
  (bind _returnvalue (Pawn|GetControlledPawn ExitingController))
  ;[1 0.3493 0] OnLogout - Removes player from PlayerController array and destroys the controlled pawn associated with the outgoing player controller
  (Utilities|IsValid _returnvalue
    (:Is%20Valid
      (Actor|DestroyActor _returnvalue))
    (:Is%20Not%20Valid
      _))
  (bind _asbp_egplayer_controller (Utilities|Casting|CastToBP_EGPlayerController ExitingController))
  (Utilities|Array|RemoveItem (Variables|Default|GetPlayer%20Controllers) _asbp_egplayer_controller))

(fn ConstructionScript)

(fn FindRandomSpawn
  (bind _outactors (Actor|GetAllActorsOfClass "/Script/Engine.PlayerStart"))
  (return (Transformation|GetActorTransform (Utilities|Array|Get(acopy) _outactors (Math|Random|RandomIntegerinRange 0 (- (Utilities|Array|Length _outactors) 1))))))

(fn SpawnPlayer
  (params (Player%20Controller :type Player%20Controller%20Object%20Reference))
  (bind _returnvalue (Pawn|GetControlledPawn Player%20Controller))
  (Utilities|IsValid _returnvalue
    (:Is%20Valid
      (Actor|DestroyActor _returnvalue))
    (:Is%20Not%20Valid
      _))
  (bind _returnvalue_2 (Game|SpawnActorfromClass "/Game/Blueprints/PlayerCharacter/BP_EGBaseCharacter.BP_EGBaseCharacter_C" (CallFunction|FindRandomSpawn) "Undefined" 0 0))
  (Pawn|Possess Player%20Controller _returnvalue_2))
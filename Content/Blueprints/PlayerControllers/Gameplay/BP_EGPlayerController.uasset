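; Multiplayer gameplay player controller that manages a player's UI, respawn requests and exits from the session.
; Tab shows the scoreboard while held, Escape or P toggles the pause menu, and events create the health widget and recolourable cursor.
; Respawn rebuilds the health widget and calls BP_GameState, replacing a deprecated GameMode path.
; Leave events destroy the pawn and disconnect through BP_BaseGI, or destroy the session and open the multiplayer menu.
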(event Custom|LeaveGame
  ;[1 1 1] Leave Game and Quit Actions
  (Game|OpenLevel(byName) "MAP_MultiplayerMenu")
  (|DestroySession self))

(event Custom|CreateCursor
  ;[0 0.8398 1] Create Cursor
  (bind _returnvalue (UserInterface|CreateWidget "/Game/Blueprints/HUD/Tools/WBP_MouseCursor.WBP_MouseCursor_C" self))
  (UserInterface|Viewport|AddtoViewport _returnvalue 1)
  (Variables|Default|SetCursorWidget _returnvalue))

(event Custom|Respawn%20Pawn
  ;[0.1335 1 0] Respawn Pawn- Requests a respawn from the server
  (Utilities|IsValid (Variables|Default|GetHealthWidget)
    (:Is%20Valid
      (Widget|RemovefromParent (Variables|Default|GetHealthWidget))
      (Variables|Default|SetHealthWidget 0))
    (:Is%20Not%20Valid
      _))
  (CallFunction|CreateHealthWidget)
  (bind _asbp_game_state (Utilities|Casting|CastToBP_GameState (Game|GetGameState)))
  (Default|GSRespawnPlayer _asbp_game_state self))

(event Custom|ExitToMainMenu
  ;[1 1 1] Leave Game and Quit Actions
  (bind _asbp_game_state (Utilities|Casting|CastToBP_GameState (Game|GetGameState)))
  (Default|GSRemovePlayerModel _asbp_game_state self))

(event Custom|KickedFromSession
  ;[1 1 1] Host Leaves Game and clients are kicked
  (|DestroySession self
    (:OnSuccess
      (Game|OpenLevel(byName) "MAP_MultiplayerMenu"))))

(event Custom|PlayerWantsToLeave
  ;[1 1 1] Client Leaves Game
  (CallFunction|ServerMakePlayerLeave))

(event Custom|CreateHealthWidget
  ;[1 0.3781 0.08416] Create Health Widget
  (Utilities|IsValid (Variables|Default|GetHealthWidget)
    (:Is%20Not%20Valid
      (bind _returnvalue (UserInterface|CreateWidget "/Game/Blueprints/HUD/Menus/WBP_HealthAndStamina.WBP_HealthAndStamina_C" self))
      (Variables|Default|SetHealthWidget _returnvalue)
      (UserInterface|Viewport|AddtoViewport _returnvalue 0))))

(event Custom|ServerMakePlayerLeave
  ;[1 1 1] Client Leaves Game
  (bind _asbp_base_gi (Utilities|Casting|CastToBP_BaseGI (Game|GetGameInstance)))
  (bind _asbp_egbase_character (Utilities|Casting|CastToBP_EGBaseCharacter (Pawn|GetControlledPawn)))
  (Actor|DestroyActor _asbp_egbase_character)
  (Default|PlayerDisconnect _asbp_base_gi self))

(event Custom|ClientLeaveSession
  ;[1 1 1] Client Leaves Game
  (|DestroySession self
    (:OnSuccess
      (Development|PrintString "Success")
      (Game|OpenLevel(byName) "MAP_MultiplayerMenu"))
    (:OnFailure
      (Development|PrintString "Failed"))))

(event Custom|ChangeCursorColour
  (params (ColourInt :type Integer))
  ;[1 1 1] Change cursor colour
  (Default|CursorColourChange (Variables|Default|GetCursorWidget) ColourInt))

(event Input|KeyboardEvents|Escape
  (params (Key :type Key%20Structure :default "None"))
  ;[0 1 0.8717] Pause Menu
  (:Pressed
    (Utilities|IsValid (Variables|Default|GetPauseWidgetInstance)
      (:Is%20Valid
        (Widget|RemovefromParent (Variables|Default|GetPauseWidgetInstance))
        (Variables|Default|SetPauseWidgetInstance 0)
        (Variables|Default|SetbShowMouseCursor false))
      (:Is%20Not%20Valid
        (bind _returnvalue (UserInterface|CreateWidget "/Game/Blueprints/HUD/Menus/WBP_PauseMenu.WBP_PauseMenu_C" self))
        (bind _output_get (Variables|Default|SetPauseWidgetInstance _returnvalue))
        (UserInterface|Viewport|AddtoViewport _returnvalue 2)
        (Variables|Default|SetbShowMouseCursor true)))))

(event Input|KeyboardEvents|P
  (params (Key :type Key%20Structure :default "None"))
  ;[0 1 0.8717] Pause Menu
  (:Pressed
    (Utilities|IsValid (Variables|Default|GetPauseWidgetInstance)
      (:Is%20Valid
        (Widget|RemovefromParent (Variables|Default|GetPauseWidgetInstance))
        (Variables|Default|SetPauseWidgetInstance 0)
        (Variables|Default|SetbShowMouseCursor false))
      (:Is%20Not%20Valid
        (bind _returnvalue (UserInterface|CreateWidget "/Game/Blueprints/HUD/Menus/WBP_PauseMenu.WBP_PauseMenu_C" self))
        (bind _output_get (Variables|Default|SetPauseWidgetInstance _returnvalue))
        (UserInterface|Viewport|AddtoViewport _returnvalue 2)
        (Variables|Default|SetbShowMouseCursor true)))))

(event Input|KeyboardEvents|Tab
  (params (Key :type Key%20Structure :default "None"))
  (:Pressed
    (Utilities|IsValid (Variables|Default|GetScoreboard)
      (:Is%20Not%20Valid
        (bind _returnvalue (UserInterface|CreateWidget "/Game/Blueprints/HUD/Menus/WBP_Scoreboard.WBP_Scoreboard_C" self))
        (bind _output_get (Variables|Default|SetScoreboard _returnvalue))
        (UserInterface|Viewport|AddtoViewport _output_get 0))))
  (:Released
    (Utilities|IsValid (Variables|Default|GetScoreboard)
      (:Is%20Valid
        (Widget|RemovefromParent (Variables|Default|GetScoreboard))
        (Variables|Default|SetScoreboard 0)))))

(fn ConstructionScript)